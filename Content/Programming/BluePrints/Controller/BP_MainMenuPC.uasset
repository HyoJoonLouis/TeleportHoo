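; BP_MainMenuPC is the main menu player controller that hosts or joins a LAN multiplayer session.
; HostSession creates a two-connection LAN session and, on success, opens L_Lobby as a listen server.
; JoinSession searches LAN sessions, stores the results and joins the first one found without checking whether the list is empty.
; Each step prints a Korean debug message, though failed searches and joins are not handled.
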(event Custom|HostSession
  (|Session self 2 true true
    (:OnSuccess
      (Development|PrintString "세션 생성")
      (Game|OpenLevel(byObjectReference) "/Game/Levels/L_Lobby.L_Lobby" true "?listen"))
    (:OnFailure
      (Development|PrintString "세션 생성 실패"))))

(event Custom|JoinSession
  (bind _results (|FindSessions self 255 true)
    (:OnSuccess
      (Development|PrintString "세션 찾음")
      (bind _output_get (Variables|Default|SetSessions _results))
      (|JoinSession self (Utilities|Array|Get(acopy) _output_get)
        (:OnSuccess
          (Development|PrintString "세션 참가"))))))

(fn ConstructionScript)
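; BP_LobbyPC is the lobby player controller, handling each player's name, ready state, character choice and lobby UI.
; SetUp creates the local lobby widget, shows Start or Leave by authority, and submits the display name.
; Name and ready changes (R key) update PlayerLobbyInfoPC through BP_LobbyGameMode, with a delayed retry event available.
; Character picks forward to the game mode; match start shows a loading screen and disables input.
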(event Custom|SelectCharacterOnServer
  (params (SelectCharacterIndex :type Integer))
  (Default|SelectCharacterClassbyIndex (Variables|Default|GetLobbyGameMode_Ref) self SelectCharacterIndex))

(event Custom|SetPlayerNameOnServer
  (params (PlayerName :type Text))
  ;[1 1 1] 쉽게 말해서 플레이어 이름 등등 세팅하고 안되면 세팅될때까지 반복해서 세팅함
  (Utilities|Struct|SetmembersinS_PlayerLobbyInfo (Variables|Default|GetPlayerLobbyInfoPC) PlayerName)
  (bind _asbp_lobby_game_mode (Utilities|Casting|CastToBP_LobbyGameMode (Game|GetGameMode)))
  (Default|UpdatePlayerLobbyInfo _asbp_lobby_game_mode self))

(event Custom|TryAgainUpdatingLobbyInfo
  ;[1 1 1] 쉽게 말해서 플레이어 이름 등등 세팅하고 안되면 세팅될때까지 반복해서 세팅함
  (Utilities|FlowControl|Delay 0.1)
  (bind _asbp_lobby_game_mode (Utilities|Casting|CastToBP_LobbyGameMode (Game|GetGameMode)))
  (Default|UpdatePlayerLobbyInfo _asbp_lobby_game_mode self))

(event Custom|ToggleReadyStatusOnServer
  (bind _playerlobbyinfopc (Variables|Default|GetPlayerLobbyInfoPC))
  (Utilities|Struct|SetmembersinS_PlayerLobbyInfo _playerlobbyinfopc (not (.bReady (Utilities|Struct|BreakS_PlayerLobbyInfo _playerlobbyinfopc))))
  (bind _asbp_lobby_game_mode (Utilities|Casting|CastToBP_LobbyGameMode (Game|GetGameMode)))
  (Default|UpdatePlayerLobbyInfo _asbp_lobby_game_mode self))

(event Custom|On%20Start%20Match
  (Default|ShowLoadingScreen (Variables|Default|GetLobbyUI_Ref_origin))
  (Input|DisableInput self))

(event EventBeginPlay
  ;[1 1 1] 쉽게 말해서 플레이어 이름 등등 세팅하고 안되면 세팅될때까지 반복해서 세팅함
  (CallFunction|SetUp)
  (Variables|Default|SetLobbyGameMode_Ref (.AsBP%20Lobby%20Game%20Mode (Utilities|Casting|CastToBP_LobbyGameMode (Game|GetGameMode)))))

(event Input|KeyboardEvents|R
  (params (Key :type Key%20Structure :default "None"))
  (:Pressed
    (CallFunction|ToggleReadyStatusonServer)))

(fn ConstructionScript)

(fn SetUp
  (if (Pawn|IsLocalPlayerController)
    (Variables|Default|SetbShowMouseCursor true)
    (Input|SetInputModeGameandUI self 0 "DoNotLock" false false)
    (bind _returnvalue (UserInterface|CreateWidget "/Game/UI/Lobby/WBP_LobbyUI_origin.WBP_LobbyUI_origin_C"))
    (bind _output_get (Variables|Default|SetLobbyUI_Ref_origin _returnvalue))
    (UserInterface|Viewport|AddtoViewport _output_get 0)
    (CallFunction|SetPlayerNameonServer (Utilities|Text|ToText(String) (Utilities|GetDisplayName (Game|GetGameInstance))))
    ;[1 1 1] 서버가 아니면 Start 버튼 안보이게
    (if (Ability|HasAuthority)
      (Widget|SetVisibility (Variables|/Game/UI/Lobby/WBP_LobbyUI_origin.WBP_LobbyUI_origin_C|GetStartButton _output_get) "Visible")
      (Widget|SetVisibility (Variables|/Game/UI/Lobby/WBP_LobbyUI_origin.WBP_LobbyUI_origin_C|GetLeaveButton _output_get) "Hidden")
      (else
        (Widget|SetVisibility (Variables|/Game/UI/Lobby/WBP_LobbyUI_origin.WBP_LobbyUI_origin_C|GetStartButton _output_get) "Hidden")
        (Widget|SetVisibility (Variables|/Game/UI/Lobby/WBP_LobbyUI_origin.WBP_LobbyUI_origin_C|GetLeaveButton _output_get) "Visible")))))
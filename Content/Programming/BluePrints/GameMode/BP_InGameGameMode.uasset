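; BP_InGameGameMode is the in-game game mode that spawns each player as the character they selected.
; It overrides GetDefaultPawnClassForController to look up the player's name in the SelectedCharactersOfAllPlayer map on BP_HooGameInstance.
; A valid class is returned as the pawn, otherwise it falls back to BP_BaseCharacter, with debug prints marking each branch.
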(event EventBeginPlay)

(event EventTick
  (params (DeltaSeconds :type Float%20%28single-precision%29)))

(fn ConstructionScript)

(fn GetDefaultPawnClassforController
  (params (InController :type Controller%20Object%20Reference))
  (bind _returnvalue (Game|GetGameInstance))
  (bind _playerstate (Variables|/Script/Engine.Controller|GetPlayerState InController))
  (bind _returnvalue_2 (PlayerState|GetPlayerName _playerstate))
  (bind _asbp_hoo_game_instance (Utilities|Casting|CastToBP_HooGameInstance _returnvalue))
  (bind _selectedcharactersofallplayer (Variables|/Game/Programming/BluePrints/BP_HooGameInstance.BP_HooGameInstance_C|GetSelectedCharactersOfAllPlayer _asbp_hoo_game_instance))
  (bind _value (Utilities|Map|Find _selectedcharactersofallplayer _returnvalue_2))
  (if (Utilities|IsValidClass _value)
    (Development|PrintString "TRUEeeeeeeeeeeeeeee ")
    (return _value)
    (else
      (Development|PrintString "falseeeeeeeeeeee")
      (return "/Game/Characters/BP_BaseCharacter.BP_BaseCharacter_C"))))
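; BP_IngameCameraManager is a player camera manager that provides a target lock-on view for BaseCharacter view targets.
; Its BlueprintUpdateCamera override keeps the FollowCamera's location and FOV but rotates the view to face TargetActor while Targeting is on and the target is valid.
; When not targeting, it returns false, leaving the view to default camera handling.
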(event EventBeginPlay)

(event Collision|EventActorBeginOverlap
  (params (OtherActor :type Actor%20Object%20Reference)))

(event EventTick
  (params (DeltaSeconds :type Float%20%28single-precision%29)))

(fn ConstructionScript)

(fn BlueprintUpdateCamera
  (params (CameraTarget :type Actor%20Object%20Reference))
  (bind _asbase_character (Utilities|Casting|CastToBaseCharacter CameraTarget))
  (if (and (Variables|/Script/TeleportHoo.BaseCharacter|GetbTargeting _asbase_character) (Utilities|IsValid (Variables|/Script/TeleportHoo.BaseCharacter|GetTargetActor _asbase_character)))
    (return (.location (Transformation|GetWorldTransform (Variables|/Script/TeleportHoo.BaseCharacter|GetFollowCamera _asbase_character))) (Math|Rotator|FindLookatRotation (.location (Transformation|GetWorldTransform (Variables|/Script/TeleportHoo.BaseCharacter|GetFollowCamera _asbase_character))) (Transformation|GetActorLocation (Variables|/Script/TeleportHoo.BaseCharacter|GetTargetActor _asbase_character))) (Variables|/Script/Engine.CameraComponent|GetFieldOfView (Variables|/Script/TeleportHoo.BaseCharacter|GetFollowCamera _asbase_character)) true)
    (else
      (return "0, 0, 0" "0, 0, 0" 0.0 false))))
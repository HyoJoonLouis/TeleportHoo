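; BP_RadialMesh is a construction-time placement actor that arranges copies of one static mesh evenly in a ring.
; The construction script adds Number + 1 mesh components, rotating a Radius vector by equal yaw steps to position each at a uniform LocalScale.
; Each copy yaws with its step, while Offset shifts only its position around the ring, not its rotation.
; The event graph holds no active logic.
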(event EventBeginPlay)

(event Collision|EventActorBeginOverlap
  (params (OtherActor :type Actor%20Object%20Reference)))

(event EventTick
  (params (DeltaSeconds :type Float%20%28single-precision%29)))

(fn ConstructionScript
  (bind _number (Variables|Default|GetNumber))
  (bind _local_scale (Variables|Default|GetLocal%20Scale))
  (for _index (range 0 _number)
    (bind _returnvalue (AddComponent|AddStaticMeshComponent false (Math|Transform|MakeTransform (Math|Vector|RotateVector (Math|Vector|MakeVector (Variables|Default|GetRadius) 0.0 0.0) (Math|Rotator|MakeRotator 0.0 0.0 (+ (Variables|Default|GetOffset) (* _index (/ 3.6e+02 (Math|Conversions|ToFloat(Integer) (+ _number 1))))))) (Math|Rotator|MakeRotator 0.0 0.0 (* _index (/ 3.6e+02 (Math|Conversions|ToFloat(Integer) (+ _number 1))))) (Math|Vector|MakeVector _local_scale _local_scale _local_scale))))
    (Components|StaticMesh|SetStaticMesh _returnvalue (Variables|Default|GetMesh))))